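; R+light is an actor with a light and an R component that continually turns relative to the player camera, like a billboard.
; Each tick it sets the whole actor's rotation so its X axis follows the vector from the camera to R, pointing away from the viewer.
; The construction script gives the light a random, very dim color by picking each RGB channel from a narrow low range.
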(event `self.ReceiveTick`
  (params (DeltaSeconds :type "Float (single-precision)"))
  (`self.SetActorRotation` (`KismetMathLibrary.MakeRotFromX` (- (`SceneComponent.K2_GetComponentLocation` (`self.R`)) (`self.K2_GetActorLocation` (`GameplayStatics.GetPlayerCameraManager` 0))))))

(fn `UserConstructionScript`
  (`LightComponent.SetLightColor` (`self.Light`) (make `LinearColor` (`KismetMathLibrary.RandomFloatInRange` 0.0 0.1) (`KismetMathLibrary.RandomFloatInRange` 0.0 0.1) (`KismetMathLibrary.RandomFloatInRange` 0.0 0.1) 1.0) true))