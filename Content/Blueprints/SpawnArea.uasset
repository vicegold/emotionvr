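; SpawnArea is an actor that spawns a letter-specific light actor for each of the A+ to Z+ input actions.
; Each press spawns that letter's class at a random point in the upper half of the Area box, offset from the actor's location, and adds it to a per-letter array.
; Release starts a one-second retriggerable delay, then destroys every actor in that array without clearing it.
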(event `InputAction|A+`
  (params (Key :type "Key Structure" :default "AnyKey"))
  (bind _spawned_a (`self.Spawned_A`))
  (bind _x (.x (`BoxComponent.GetScaledBoxExtent` (`self.Area`))))
  (bind _y (.y (`BoxComponent.GetScaledBoxExtent` (`self.Area`))))
  (bind _z (.z (`BoxComponent.GetScaledBoxExtent` (`self.Area`))))
  (:`Pressed`
    (bind _returnvalue (`|SpawnActorFromClass` "/Game/Blueprints/A+light.A+light_C" (`KismetMathLibrary.MakeTransform` (+ (`KismetMathLibrary.MakeVector` (`KismetMathLibrary.RandomFloatInRange` (* _x -1.0) _x) (`KismetMathLibrary.RandomFloatInRange` (* _y -1.0) _y) (`KismetMathLibrary.RandomFloatInRange` (* 0.0 _z) _z)) (`self.K2_GetActorLocation`))) "Undefined" "OverrideRootScale"))
    (`KismetArrayLibrary.Array_Add` _spawned_a _returnvalue))
  (:`Released`
    (`KismetSystemLibrary.RetriggerableDelay` 1.0)
    (`self.K2_DestroyActor` _spawned_a)))

(event `InputAction|B+`
  (params (Key :type "Key Structure" :default "AnyKey"))
  (bind _spawned_b (`self.Spawned_B`))
  (bind _x (.x (`BoxComponent.GetScaledBoxExtent` (`self.Area`))))
  (bind _y (.y (`BoxComponent.GetScaledBoxExtent` (`self.Area`))))
  (bind _z (.z (`BoxComponent.GetScaledBoxExtent` (`self.Area`))))
  (:`Pressed`
    (bind _returnvalue (`|SpawnActorFromClass` "/Game/Blueprints/B+light.B+light_C" (`KismetMathLibrary.MakeTransform` (+ (`KismetMathLibrary.MakeVector` (`KismetMathLibrary.RandomFloatInRange` (* _x -1.0) _x) (`KismetMathLibrary.RandomFloatInRange` (* _y -1.0) _y) (`KismetMathLibrary.RandomFloatInRange` (* 0.0 _z) _z)) (`self.K2_GetActorLocation`))) "Undefined" "OverrideRootScale"))
    (`KismetArrayLibrary.Array_Add` _spawned_b _returnvalue))
  (:`Released`
    (`KismetSystemLibrary.RetriggerableDelay` 1.0)
    (`self.K2_DestroyActor` _spawned_b)))

(event `InputAction|C+`
  (params (Key :type "Key Structure" :default "AnyKey"))
  (bind _spawned_c (`self.Spawned_C`))
  (bind _x (.x (`BoxComponent.GetScaledBoxExtent` (`self.Area`))))
  (bind _y (.y (`BoxComponent.GetScaledBoxExtent` (`self.Area`))))
  (bind _z (.z (`BoxComponent.GetScaledBoxExtent` (`self.Area`))))
  (:`Pressed`
    (bind _returnvalue (`|SpawnActorFromClass` "/Game/Blueprints/C+light.C+light_C" (`KismetMathLibrary.MakeTransform` (+ (`KismetMathLibrary.MakeVector` (`KismetMathLibrary.RandomFloatInRange` (* _x -1.0) _x) (`KismetMathLibrary.RandomFloatInRange` (* _y -1.0) _y) (`KismetMathLibrary.RandomFloatInRange` (* 0.0 _z) _z)) (`self.K2_GetActorLocation`))) "Undefined" "OverrideRootScale"))
    (`KismetArrayLibrary.Array_Add` _spawned_c _returnvalue))
  (:`Released`
    (`KismetSystemLibrary.RetriggerableDelay` 1.0)
    (`self.K2_DestroyActor` _spawned_c)))

(event `InputAction|D+`
  (params (Key :type "Key Structure" :default "AnyKey"))
  (bind _spawned_d (`self.Spawned_D`))
  (bind _x (.x (`BoxComponent.GetScaledBoxExtent` (`self.Area`))))
  (bind _y (.y (`BoxComponent.GetScaledBoxExtent` (`self.Area`))))
  (bind _z (.z (`BoxComponent.GetScaledBoxExtent` (`self.Area`))))
  (:`Pressed`
    (bind _returnvalue (`|SpawnActorFromClass` "/Game/Blueprints/D+light.D+light_C" (`KismetMathLibrary.MakeTransform` (+ (`KismetMathLibrary.MakeVector` (`KismetMathLibrary.RandomFloatInRange` (* _x -1.0) _x) (`KismetMathLibrary.RandomFloatInRange` (* _y -1.0) _y) (`KismetMathLibrary.RandomFloatInRange` (* 0.0 _z) _z)) (`self.K2_GetActorLocation`))) "Undefined" "OverrideRootScale"))
    (`KismetArrayLibrary.Array_Add` _spawned_d _returnvalue))
  (:`Released`
    (`KismetSystemLibrary.RetriggerableDelay` 1.0)
    (`self.K2_DestroyActor` _spawned_d)))

(event `InputAction|E+`
  (params (Key :type "Key Structure" :default "AnyKey"))
  (bind _spawned_e (`self.Spawned_E`))
  (bind _x (.x (`BoxComponent.GetScaledBoxExtent` (`self.Area`))))
  (bind _y (.y (`BoxComponent.GetScaledBoxExtent` (`self.Area`))))
  (bind _z (.z (`BoxComponent.GetScaledBoxExtent` (`self.Area`))))
  (:`Pressed`
    (bind _returnvalue (`|SpawnActorFromClass` "/Game/Blueprints/E+light.E+light_C" (`KismetMathLibrary.MakeTransform` (+ (`KismetMathLibrary.MakeVector` (`KismetMathLibrary.RandomFloatInRange` (* _x -1.0) _x) (`KismetMathLibrary.RandomFloatInRange` (* _y -1.0) _y) (`KismetMathLibrary.RandomFloatInRange` (* 0.0 _z) _z)) (`self.K2_GetActorLocation`))) "Undefined" "OverrideRootScale"))
    (`KismetArrayLibrary.Array_Add` _spawned_e _returnvalue))
  (:`Released`
    (`KismetSystemLibrary.RetriggerableDelay` 1.0)
    (`self.K2_DestroyActor` _spawned_e)))

(event `InputAction|F+`
  (params (Key :type "Key Structure" :default "AnyKey"))
  (bind _spawned_f (`self.Spawned_F`))
  (bind _x (.x (`BoxComponent.GetScaledBoxExtent` (`self.Area`))))
  (bind _y (.y (`BoxComponent.GetScaledBoxExtent` (`self.Area`))))
  (bind _z (.z (`BoxComponent.GetScaledBoxExtent` (`self.Area`))))
  (:`Pressed`
    (bind _returnvalue (`|SpawnActorFromClass` "/Game/Blueprints/F+light.F+light_C" (`KismetMathLibrary.MakeTransform` (+ (`KismetMathLibrary.MakeVector` (`KismetMathLibrary.RandomFloatInRange` (* _x -1.0) _x) (`KismetMathLibrary.RandomFloatInRange` (* _y -1.0) _y) (`KismetMathLibrary.RandomFloatInRange` (* 0.0 _z) _z)) (`self.K2_GetActorLocation`))) "Undefined" "OverrideRootScale"))
    (`KismetArrayLibrary.Array_Add` _spawned_f _returnvalue))
  (:`Released`
    (`KismetSystemLibrary.RetriggerableDelay` 1.0)
    (`self.K2_DestroyActor` _spawned_f)))

(event `InputAction|G+`
  (params (Key :type "Key Structure" :default "AnyKey"))
  (bind _spawned_g (`self.Spawned_G`))
  (bind _x (.x (`BoxComponent.GetScaledBoxExtent` (`self.Area`))))
  (bind _y (.y (`BoxComponent.GetScaledBoxExtent` (`self.Area`))))
  (bind _z (.z (`BoxComponent.GetScaledBoxExtent` (`self.Area`))))
  (:`Pressed`
    (bind _returnvalue (`|SpawnActorFromClass` "/Game/Blueprints/G+light.G+light_C" (`KismetMathLibrary.MakeTransform` (+ (`KismetMathLibrary.MakeVector` (`KismetMathLibrary.RandomFloatInRange` (* _x -1.0) _x) (`KismetMathLibrary.RandomFloatInRange` (* _y -1.0) _y) (`KismetMathLibrary.RandomFloatInRange` (* 0.0 _z) _z)) (`self.K2_GetActorLocation`))) "Undefined" "OverrideRootScale"))
    (`KismetArrayLibrary.Array_Add` _spawned_g _returnvalue))
  (:`Released`
    (`KismetSystemLibrary.RetriggerableDelay` 1.0)
    (`self.K2_DestroyActor` _spawned_g)))

(event `InputAction|H+`
  (params (Key :type "Key Structure" :default "AnyKey"))
  (bind _spawned_h (`self.Spawned_H`))
  (bind _x (.x (`BoxComponent.GetScaledBoxExtent` (`self.Area`))))
  (bind _y (.y (`BoxComponent.GetScaledBoxExtent` (`self.Area`))))
  (bind _z (.z (`BoxComponent.GetScaledBoxExtent` (`self.Area`))))
  (:`Pressed`
    (bind _returnvalue (`|SpawnActorFromClass` "/Game/Blueprints/H+light.H+light_C" (`KismetMathLibrary.MakeTransform` (+ (`KismetMathLibrary.MakeVector` (`KismetMathLibrary.RandomFloatInRange` (* _x -1.0) _x) (`KismetMathLibrary.RandomFloatInRange` (* _y -1.0) _y) (`KismetMathLibrary.RandomFloatInRange` (* 0.0 _z) _z)) (`self.K2_GetActorLocation`))) "Undefined" "OverrideRootScale"))
    (`KismetArrayLibrary.Array_Add` _spawned_h _returnvalue))
  (:`Released`
    (`KismetSystemLibrary.RetriggerableDelay` 1.0)
    (`self.K2_DestroyActor` _spawned_h)))

(event `InputAction|I+`
  (params (Key :type "Key Structure" :default "AnyKey"))
  (bind _spawned_i (`self.Spawned_I`))
  (bind _x (.x (`BoxComponent.GetScaledBoxExtent` (`self.Area`))))
  (bind _y (.y (`BoxComponent.GetScaledBoxExtent` (`self.Area`))))
  (bind _z (.z (`BoxComponent.GetScaledBoxExtent` (`self.Area`))))
  (:`Pressed`
    (bind _returnvalue (`|SpawnActorFromClass` "/Game/Blueprints/I+light.I+light_C" (`KismetMathLibrary.MakeTransform` (+ (`KismetMathLibrary.MakeVector` (`KismetMathLibrary.RandomFloatInRange` (* _x -1.0) _x) (`KismetMathLibrary.RandomFloatInRange` (* _y -1.0) _y) (`KismetMathLibrary.RandomFloatInRange` (* 0.0 _z) _z)) (`self.K2_GetActorLocation`))) "Undefined" "OverrideRootScale"))
    (`KismetArrayLibrary.Array_Add` _spawned_i _returnvalue))
  (:`Released`
    (`KismetSystemLibrary.RetriggerableDelay` 1.0)
    (`self.K2_DestroyActor` _spawned_i)))

(event `InputAction|J+`
  (params (Key :type "Key Structure" :default "AnyKey"))
  (bind _spawned_j (`self.Spawned_J`))
  (bind _x (.x (`BoxComponent.GetScaledBoxExtent` (`self.Area`))))
  (bind _y (.y (`BoxComponent.GetScaledBoxExtent` (`self.Area`))))
  (bind _z (.z (`BoxComponent.GetScaledBoxExtent` (`self.Area`))))
  (:`Pressed`
    (bind _returnvalue (`|SpawnActorFromClass` "/Game/Blueprints/J+light.J+light_C" (`KismetMathLibrary.MakeTransform` (+ (`KismetMathLibrary.MakeVector` (`KismetMathLibrary.RandomFloatInRange` (* _x -1.0) _x) (`KismetMathLibrary.RandomFloatInRange` (* _y -1.0) _y) (`KismetMathLibrary.RandomFloatInRange` (* 0.0 _z) _z)) (`self.K2_GetActorLocation`))) "Undefined" "OverrideRootScale"))
    (`KismetArrayLibrary.Array_Add` _spawned_j _returnvalue))
  (:`Released`
    (`KismetSystemLibrary.RetriggerableDelay` 1.0)
    (`self.K2_DestroyActor` _spawned_j)))

(event `InputAction|K+`
  (params (Key :type "Key Structure" :default "AnyKey"))
  (bind _spawned_k (`self.Spawned_K`))
  (bind _x (.x (`BoxComponent.GetScaledBoxExtent` (`self.Area`))))
  (bind _y (.y (`BoxComponent.GetScaledBoxExtent` (`self.Area`))))
  (bind _z (.z (`BoxComponent.GetScaledBoxExtent` (`self.Area`))))
  (:`Pressed`
    (bind _returnvalue (`|SpawnActorFromClass` "/Game/Blueprints/K+light.K+light_C" (`KismetMathLibrary.MakeTransform` (+ (`KismetMathLibrary.MakeVector` (`KismetMathLibrary.RandomFloatInRange` (* _x -1.0) _x) (`KismetMathLibrary.RandomFloatInRange` (* _y -1.0) _y) (`KismetMathLibrary.RandomFloatInRange` (* 0.0 _z) _z)) (`self.K2_GetActorLocation`))) "Undefined" "OverrideRootScale"))
    (`KismetArrayLibrary.Array_Add` _spawned_k _returnvalue))
  (:`Released`
    (`KismetSystemLibrary.RetriggerableDelay` 1.0)
    (`self.K2_DestroyActor` _spawned_k)))

(event `InputAction|L+`
  (params (Key :type "Key Structure" :default "AnyKey"))
  (bind _spawned_l (`self.Spawned_L`))
  (bind _x (.x (`BoxComponent.GetScaledBoxExtent` (`self.Area`))))
  (bind _y (.y (`BoxComponent.GetScaledBoxExtent` (`self.Area`))))
  (bind _z (.z (`BoxComponent.GetScaledBoxExtent` (`self.Area`))))
  (:`Pressed`
    (bind _returnvalue (`|SpawnActorFromClass` "/Game/Blueprints/L+light.L+light_C" (`KismetMathLibrary.MakeTransform` (+ (`KismetMathLibrary.MakeVector` (`KismetMathLibrary.RandomFloatInRange` (* _x -1.0) _x) (`KismetMathLibrary.RandomFloatInRange` (* _y -1.0) _y) (`KismetMathLibrary.RandomFloatInRange` (* 0.0 _z) _z)) (`self.K2_GetActorLocation`))) "Undefined" "OverrideRootScale"))
    (`KismetArrayLibrary.Array_Add` _spawned_l _returnvalue))
  (:`Released`
    (`KismetSystemLibrary.RetriggerableDelay` 1.0)
    (`self.K2_DestroyActor` _spawned_l)))

(event `InputAction|M+`
  (params (Key :type "Key Structure" :default "AnyKey"))
  (bind _spawned_m (`self.Spawned_M`))
  (bind _x (.x (`BoxComponent.GetScaledBoxExtent` (`self.Area`))))
  (bind _y (.y (`BoxComponent.GetScaledBoxExtent` (`self.Area`))))
  (bind _z (.z (`BoxComponent.GetScaledBoxExtent` (`self.Area`))))
  (:`Pressed`
    (bind _returnvalue (`|SpawnActorFromClass` "/Game/Blueprints/M+light.M+light_C" (`KismetMathLibrary.MakeTransform` (+ (`KismetMathLibrary.MakeVector` (`KismetMathLibrary.RandomFloatInRange` (* _x -1.0) _x) (`KismetMathLibrary.RandomFloatInRange` (* _y -1.0) _y) (`KismetMathLibrary.RandomFloatInRange` (* 0.0 _z) _z)) (`self.K2_GetActorLocation`))) "Undefined" "OverrideRootScale"))
    (`KismetArrayLibrary.Array_Add` _spawned_m _returnvalue))
  (:`Released`
    (`KismetSystemLibrary.RetriggerableDelay` 1.0)
    (`self.K2_DestroyActor` _spawned_m)))

(event `InputAction|N+`
  (params (Key :type "Key Structure" :default "AnyKey"))
  (bind _spawned_n (`self.Spawned_N`))
  (bind _x (.x (`BoxComponent.GetScaledBoxExtent` (`self.Area`))))
  (bind _y (.y (`BoxComponent.GetScaledBoxExtent` (`self.Area`))))
  (bind _z (.z (`BoxComponent.GetScaledBoxExtent` (`self.Area`))))
  (:`Pressed`
    (bind _returnvalue (`|SpawnActorFromClass` "/Game/Blueprints/N+light.N+light_C" (`KismetMathLibrary.MakeTransform` (+ (`KismetMathLibrary.MakeVector` (`KismetMathLibrary.RandomFloatInRange` (* _x -1.0) _x) (`KismetMathLibrary.RandomFloatInRange` (* _y -1.0) _y) (`KismetMathLibrary.RandomFloatInRange` (* 0.0 _z) _z)) (`self.K2_GetActorLocation`))) "Undefined" "OverrideRootScale"))
    (`KismetArrayLibrary.Array_Add` _spawned_n _returnvalue))
  (:`Released`
    (`KismetSystemLibrary.RetriggerableDelay` 1.0)
    (`self.K2_DestroyActor` _spawned_n)))

(event `InputAction|O+`
  (params (Key :type "Key Structure" :default "AnyKey"))
  (bind _spawned_o (`self.Spawned_O`))
  (bind _x (.x (`BoxComponent.GetScaledBoxExtent` (`self.Area`))))
  (bind _y (.y (`BoxComponent.GetScaledBoxExtent` (`self.Area`))))
  (bind _z (.z (`BoxComponent.GetScaledBoxExtent` (`self.Area`))))
  (:`Pressed`
    (bind _returnvalue (`|SpawnActorFromClass` "/Game/Blueprints/O+light.O+light_C" (`KismetMathLibrary.MakeTransform` (+ (`KismetMathLibrary.MakeVector` (`KismetMathLibrary.RandomFloatInRange` (* _x -1.0) _x) (`KismetMathLibrary.RandomFloatInRange` (* _y -1.0) _y) (`KismetMathLibrary.RandomFloatInRange` (* 0.0 _z) _z)) (`self.K2_GetActorLocation`))) "Undefined" "OverrideRootScale"))
    (`KismetArrayLibrary.Array_Add` _spawned_o _returnvalue))
  (:`Released`
    (`KismetSystemLibrary.RetriggerableDelay` 1.0)
    (`self.K2_DestroyActor` _spawned_o)))

(event `InputAction|P+`
  (params (Key :type "Key Structure" :default "AnyKey"))
  (bind _spawned_p (`self.Spawned_P`))
  (bind _x (.x (`BoxComponent.GetScaledBoxExtent` (`self.Area`))))
  (bind _y (.y (`BoxComponent.GetScaledBoxExtent` (`self.Area`))))
  (bind _z (.z (`BoxComponent.GetScaledBoxExtent` (`self.Area`))))
  (:`Pressed`
    (bind _returnvalue (`|SpawnActorFromClass` "/Game/Blueprints/P+light.P+light_C" (`KismetMathLibrary.MakeTransform` (+ (`KismetMathLibrary.MakeVector` (`KismetMathLibrary.RandomFloatInRange` (* _x -1.0) _x) (`KismetMathLibrary.RandomFloatInRange` (* _y -1.0) _y) (`KismetMathLibrary.RandomFloatInRange` (* 0.0 _z) _z)) (`self.K2_GetActorLocation`))) "Undefined" "OverrideRootScale"))
    (`KismetArrayLibrary.Array_Add` _spawned_p _returnvalue))
  (:`Released`
    (`KismetSystemLibrary.RetriggerableDelay` 1.0)
    (`self.K2_DestroyActor` _spawned_p)))

(event `InputAction|Q+`
  (params (Key :type "Key Structure" :default "AnyKey"))
  (bind _spawned_q (`self.Spawned_Q`))
  (bind _x (.x (`BoxComponent.GetScaledBoxExtent` (`self.Area`))))
  (bind _y (.y (`BoxComponent.GetScaledBoxExtent` (`self.Area`))))
  (bind _z (.z (`BoxComponent.GetScaledBoxExtent` (`self.Area`))))
  (:`Pressed`
    (bind _returnvalue (`|SpawnActorFromClass` "/Game/Blueprints/Q+light.Q+light_C" (`KismetMathLibrary.MakeTransform` (+ (`KismetMathLibrary.MakeVector` (`KismetMathLibrary.RandomFloatInRange` (* _x -1.0) _x) (`KismetMathLibrary.RandomFloatInRange` (* _y -1.0) _y) (`KismetMathLibrary.RandomFloatInRange` (* 0.0 _z) _z)) (`self.K2_GetActorLocation`))) "Undefined" "OverrideRootScale"))
    (`KismetArrayLibrary.Array_Add` _spawned_q _returnvalue))
  (:`Released`
    (`KismetSystemLibrary.RetriggerableDelay` 1.0)
    (`self.K2_DestroyActor` _spawned_q)))

(event `InputAction|R+`
  (params (Key :type "Key Structure" :default "AnyKey"))
  (bind _spawned_r (`self.Spawned_R`))
  (bind _x (.x (`BoxComponent.GetScaledBoxExtent` (`self.Area`))))
  (bind _y (.y (`BoxComponent.GetScaledBoxExtent` (`self.Area`))))
  (bind _z (.z (`BoxComponent.GetScaledBoxExtent` (`self.Area`))))
  (:`Pressed`
    (bind _returnvalue (`|SpawnActorFromClass` "/Game/Blueprints/R+light.R+light_C" (`KismetMathLibrary.MakeTransform` (+ (`KismetMathLibrary.MakeVector` (`KismetMathLibrary.RandomFloatInRange` (* _x -1.0) _x) (`KismetMathLibrary.RandomFloatInRange` (* _y -1.0) _y) (`KismetMathLibrary.RandomFloatInRange` (* 0.0 _z) _z)) (`self.K2_GetActorLocation`))) "Undefined" "OverrideRootScale"))
    (`KismetArrayLibrary.Array_Add` _spawned_r _returnvalue))
  (:`Released`
    (`KismetSystemLibrary.RetriggerableDelay` 1.0)
    (`self.K2_DestroyActor` _spawned_r)))

(event `InputAction|S+`
  (params (Key :type "Key Structure" :default "AnyKey"))
  (bind _spawned_s (`self.Spawned_S`))
  (bind _x (.x (`BoxComponent.GetScaledBoxExtent` (`self.Area`))))
  (bind _y (.y (`BoxComponent.GetScaledBoxExtent` (`self.Area`))))
  (bind _z (.z (`BoxComponent.GetScaledBoxExtent` (`self.Area`))))
  (:`Pressed`
    (bind _returnvalue (`|SpawnActorFromClass` "/Game/Blueprints/S+light.S+light_C" (`KismetMathLibrary.MakeTransform` (+ (`KismetMathLibrary.MakeVector` (`KismetMathLibrary.RandomFloatInRange` (* _x -1.0) _x) (`KismetMathLibrary.RandomFloatInRange` (* _y -1.0) _y) (`KismetMathLibrary.RandomFloatInRange` (* 0.0 _z) _z)) (`self.K2_GetActorLocation`))) "Undefined" "OverrideRootScale"))
    (`KismetArrayLibrary.Array_Add` _spawned_s _returnvalue))
  (:`Released`
    (`KismetSystemLibrary.RetriggerableDelay` 1.0)
    (`self.K2_DestroyActor` _spawned_s)))

(event `InputAction|T+`
  (params (Key :type "Key Structure" :default "AnyKey"))
  (bind _spawned_t (`self.Spawned_T`))
  (bind _x (.x (`BoxComponent.GetScaledBoxExtent` (`self.Area`))))
  (bind _y (.y (`BoxComponent.GetScaledBoxExtent` (`self.Area`))))
  (bind _z (.z (`BoxComponent.GetScaledBoxExtent` (`self.Area`))))
  (:`Pressed`
    (bind _returnvalue (`|SpawnActorFromClass` "/Game/Blueprints/T+light.T+light_C" (`KismetMathLibrary.MakeTransform` (+ (`KismetMathLibrary.MakeVector` (`KismetMathLibrary.RandomFloatInRange` (* _x -1.0) _x) (`KismetMathLibrary.RandomFloatInRange` (* _y -1.0) _y) (`KismetMathLibrary.RandomFloatInRange` (* 0.0 _z) _z)) (`self.K2_GetActorLocation`))) "Undefined" "OverrideRootScale"))
    (`KismetArrayLibrary.Array_Add` _spawned_t _returnvalue))
  (:`Released`
    (`KismetSystemLibrary.RetriggerableDelay` 1.0)
    (`self.K2_DestroyActor` _spawned_t)))

(event `InputAction|U+`
  (params (Key :type "Key Structure" :default "AnyKey"))
  (bind _spawned_u (`self.Spawned_U`))
  (bind _x (.x (`BoxComponent.GetScaledBoxExtent` (`self.Area`))))
  (bind _y (.y (`BoxComponent.GetScaledBoxExtent` (`self.Area`))))
  (bind _z (.z (`BoxComponent.GetScaledBoxExtent` (`self.Area`))))
  (:`Pressed`
    (bind _returnvalue (`|SpawnActorFromClass` "/Game/Blueprints/U+light.U+light_C" (`KismetMathLibrary.MakeTransform` (+ (`KismetMathLibrary.MakeVector` (`KismetMathLibrary.RandomFloatInRange` (* _x -1.0) _x) (`KismetMathLibrary.RandomFloatInRange` (* _y -1.0) _y) (`KismetMathLibrary.RandomFloatInRange` (* 0.0 _z) _z)) (`self.K2_GetActorLocation`))) "Undefined" "OverrideRootScale"))
    (`KismetArrayLibrary.Array_Add` _spawned_u _returnvalue))
  (:`Released`
    (`KismetSystemLibrary.RetriggerableDelay` 1.0)
    (`self.K2_DestroyActor` _spawned_u)))

(event `InputAction|V+`
  (params (Key :type "Key Structure" :default "AnyKey"))
  (bind _spawned_v (`self.Spawned_V`))
  (bind _x (.x (`BoxComponent.GetScaledBoxExtent` (`self.Area`))))
  (bind _y (.y (`BoxComponent.GetScaledBoxExtent` (`self.Area`))))
  (bind _z (.z (`BoxComponent.GetScaledBoxExtent` (`self.Area`))))
  (:`Pressed`
    (bind _returnvalue (`|SpawnActorFromClass` "/Game/Blueprints/V+light.V+light_C" (`KismetMathLibrary.MakeTransform` (+ (`KismetMathLibrary.MakeVector` (`KismetMathLibrary.RandomFloatInRange` (* _x -1.0) _x) (`KismetMathLibrary.RandomFloatInRange` (* _y -1.0) _y) (`KismetMathLibrary.RandomFloatInRange` (* 0.0 _z) _z)) (`self.K2_GetActorLocation`))) "Undefined" "OverrideRootScale"))
    (`KismetArrayLibrary.Array_Add` _spawned_v _returnvalue))
  (:`Released`
    (`KismetSystemLibrary.RetriggerableDelay` 1.0)
    (`self.K2_DestroyActor` _spawned_v)))

(event `InputAction|W+`
  (params (Key :type "Key Structure" :default "AnyKey"))
  (bind _spawned_w (`self.Spawned_W`))
  (bind _x (.x (`BoxComponent.GetScaledBoxExtent` (`self.Area`))))
  (bind _y (.y (`BoxComponent.GetScaledBoxExtent` (`self.Area`))))
  (bind _z (.z (`BoxComponent.GetScaledBoxExtent` (`self.Area`))))
  (:`Pressed`
    (bind _returnvalue (`|SpawnActorFromClass` "/Game/Blueprints/W+light.W+light_C" (`KismetMathLibrary.MakeTransform` (+ (`KismetMathLibrary.MakeVector` (`KismetMathLibrary.RandomFloatInRange` (* _x -1.0) _x) (`KismetMathLibrary.RandomFloatInRange` (* _y -1.0) _y) (`KismetMathLibrary.RandomFloatInRange` (* 0.0 _z) _z)) (`self.K2_GetActorLocation`))) "Undefined" "OverrideRootScale"))
    (`KismetArrayLibrary.Array_Add` _spawned_w _returnvalue))
  (:`Released`
    (`KismetSystemLibrary.RetriggerableDelay` 1.0)
    (`self.K2_DestroyActor` _spawned_w)))

(event `InputAction|X+`
  (params (Key :type "Key Structure" :default "AnyKey"))
  (bind _spawned_x (`self.Spawned_X`))
  (bind _x (.x (`BoxComponent.GetScaledBoxExtent` (`self.Area`))))
  (bind _y (.y (`BoxComponent.GetScaledBoxExtent` (`self.Area`))))
  (bind _z (.z (`BoxComponent.GetScaledBoxExtent` (`self.Area`))))
  (:`Pressed`
    (bind _returnvalue (`|SpawnActorFromClass` "/Game/Blueprints/X+light.X+light_C" (`KismetMathLibrary.MakeTransform` (+ (`KismetMathLibrary.MakeVector` (`KismetMathLibrary.RandomFloatInRange` (* _x -1.0) _x) (`KismetMathLibrary.RandomFloatInRange` (* _y -1.0) _y) (`KismetMathLibrary.RandomFloatInRange` (* 0.0 _z) _z)) (`self.K2_GetActorLocation`))) "Undefined" "OverrideRootScale"))
    (`KismetArrayLibrary.Array_Add` _spawned_x _returnvalue))
  (:`Released`
    (`KismetSystemLibrary.RetriggerableDelay` 1.0)
    (`self.K2_DestroyActor` _spawned_x)))

(event `InputAction|Y+`
  (params (Key :type "Key Structure" :default "AnyKey"))
  (bind _spawned_y (`self.Spawned_Y`))
  (bind _x (.x (`BoxComponent.GetScaledBoxExtent` (`self.Area`))))
  (bind _y (.y (`BoxComponent.GetScaledBoxExtent` (`self.Area`))))
  (bind _z (.z (`BoxComponent.GetScaledBoxExtent` (`self.Area`))))
  (:`Pressed`
    (bind _returnvalue (`|SpawnActorFromClass` "/Game/Blueprints/Y+light.Y+light_C" (`KismetMathLibrary.MakeTransform` (+ (`KismetMathLibrary.MakeVector` (`KismetMathLibrary.RandomFloatInRange` (* _x -1.0) _x) (`KismetMathLibrary.RandomFloatInRange` (* _y -1.0) _y) (`KismetMathLibrary.RandomFloatInRange` (* 0.0 _z) _z)) (`self.K2_GetActorLocation`))) "Undefined" "OverrideRootScale"))
    (`KismetArrayLibrary.Array_Add` _spawned_y _returnvalue))
  (:`Released`
    (`KismetSystemLibrary.RetriggerableDelay` 1.0)
    (`self.K2_DestroyActor` _spawned_y)))

(event `InputAction|Z+`
  (params (Key :type "Key Structure" :default "AnyKey"))
  (bind _spawned_z (`self.Spawned_Z`))
  (bind _x (.x (`BoxComponent.GetScaledBoxExtent` (`self.Area`))))
  (bind _y (.y (`BoxComponent.GetScaledBoxExtent` (`self.Area`))))
  (bind _z (.z (`BoxComponent.GetScaledBoxExtent` (`self.Area`))))
  (:`Pressed`
    (bind _returnvalue (`|SpawnActorFromClass` "/Game/Blueprints/Z+light.Z+light_C" (`KismetMathLibrary.MakeTransform` (+ (`KismetMathLibrary.MakeVector` (`KismetMathLibrary.RandomFloatInRange` (* _x -1.0) _x) (`KismetMathLibrary.RandomFloatInRange` (* _y -1.0) _y) (`KismetMathLibrary.RandomFloatInRange` (* 0.0 _z) _z)) (`self.K2_GetActorLocation`))) "Undefined" "OverrideRootScale"))
    (`KismetArrayLibrary.Array_Add` _spawned_z _returnvalue))
  (:`Released`
    (`KismetSystemLibrary.RetriggerableDelay` 1.0)
    (`self.K2_DestroyActor` _spawned_z)))

(fn `UserConstructionScript`)